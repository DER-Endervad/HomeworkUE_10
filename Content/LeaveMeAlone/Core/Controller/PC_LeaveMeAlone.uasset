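; Player controller for LeaveMeAlone that handles the pause menu and the death screen.
; Pause input, guarded by OnPause, pauses the game and shows WBP_Pause with UI-only input; a custom event does the same without the guard.
; UnPossess passes the cached CH_Player's score to WBP_Death and starts a looping one-second timer.
; When the TimerForDeath countdown hits zero, the game pauses, the death widget appears and a sound plays.
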(event Custom|CustomEvent
  (Game|SetGamePaused true)
  (bind _returnvalue (UserInterface|CreateWidget "/Game/LeaveMeAlone/UI/WBP_Pause.WBP_Pause_C"))
  (bind _output_get (Variables|Default|SetPause%20Widget _returnvalue))
  (UserInterface|Viewport|AddtoViewport _output_get 0)
  (Input|SetInputModeUIOnly self _output_get "DoNotLock" false)
  (Variables|Default|SetbShowMouseCursor true))

(event Custom|TimerEvent
  (bind _self self)
  (bind _death_widget (Variables|Default|GetDeath%20Widget))
  (bind _result (Math|Integer|DecrementInt (Variables|Default|GetTimerForDeath))
    (:%20%20
      (if (== _result 0)
        (Game|SetGamePaused true)
        (UserInterface|Viewport|AddtoViewport _death_widget 0)
        (Input|SetInputModeUIOnly _self _death_widget "DoNotLock" false)
        (Variables|/Script/Engine.PlayerController|SetbShowMouseCursor _self true)
        (Audio|PlaySound2D "/Game/LeaveMeAlone/Audio/Death.Death" 1.0 1.0 0.0 0 0)))))

(event EventBeginPlay
  (bind _asch_player (Utilities|Casting|CastToCH_Player (Game|GetPlayerCharacter 0)))
  (Variables|Default|SetAs%20CH%20Player _asch_player))

(event EventTick
  (params (DeltaSeconds :type Float%20%28single-precision%29)))

(event EventUnPossess
  (params (UnpossessedPawn :type Pawn%20Object%20Reference))
  (bind _returnvalue (UserInterface|CreateWidget "/Game/LeaveMeAlone/UI/WBP_Death.WBP_Death_C"))
  (bind _output_get (Variables|Default|SetDeath%20Widget _returnvalue))
  (Default|AddScore _output_get (Variables|/Game/LeaveMeAlone/Core/Character/CH_Player.CH_Player_C|GetScore (Variables|Default|GetAs%20CH%20Player)))
  (bind _returnvalue_2 (Utilities|Time|SetTimerbyEvent (EventDispatchers|CreateEvent :!event Custom|TimerEvent) 1.0 true))
  (Variables|Default|SetTimer _returnvalue_2))

(event Input|ActionEvents|InputActionPause
  (params (Key :type Key%20Structure :default "None"))
  (:Pressed
    (if (not (Variables|Default|GetOnPause))
      (Variables|Default|SetOnPause true)
      (Game|SetGamePaused true)
      (bind _returnvalue (UserInterface|CreateWidget "/Game/LeaveMeAlone/UI/WBP_Pause.WBP_Pause_C"))
      (bind _output_get (Variables|Default|SetPause%20Widget _returnvalue))
      (UserInterface|Viewport|AddtoViewport _output_get 0)
      (Input|SetInputModeUIOnly self _output_get "DoNotLock" false)
      (Variables|Default|SetbShowMouseCursor true))))

(fn ConstructionScript)